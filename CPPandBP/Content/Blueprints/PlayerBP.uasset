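; Player pawn Blueprint that handles look, movement, interaction and UI input.
; Movement follows control yaw only, and the forward and right axis values are also stored in variables.
; BeginPlay creates the MainGUI widget, which the Inventory and Menu actions toggle, with Menu also switching cursor visibility and game-only or UI-only input mode.
; Interact calls an Interaction function not defined in this graph, and Debug flips a flag.
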(event EventBeginPlay
  (bind _returnvalue (UserInterface|CreateWidget "/Game/GUI/MainGUI.MainGUI_C"))
  (bind _output_get (Variables|Default|SetMainGUI _returnvalue))
  (UserInterface|Viewport|AddtoViewport _output_get 0))

(event Input|ActionEvents|InputActionInteract
  (params (Key :type Key%20Structure :default "None"))
  (:Pressed
    (Class|PlayerCharacterCPP|Interaction)))

(event Input|ActionEvents|InputActionInventory
  (params (Key :type Key%20Structure :default "None"))
  (:Pressed
    (Class|MainGUICPP|ToggleInventoryVisibility (Variables|Default|GetMainGUI))))

(event Input|ActionEvents|InputActionMenu
  (params (Key :type Key%20Structure :default "None"))
  (bind _returnvalue (Game|GetPlayerController 0))
  (bind _maingui (Variables|Default|GetMainGUI))
  (:Pressed
    (bind _returnvalue_2 (Class|MainGUICPP|ToggleMenuVisibility _maingui))
    (Variables|/Script/Engine.PlayerController|SetbShowMouseCursor _returnvalue (not _returnvalue_2))
    (if _returnvalue_2
      (Input|SetInputModeGameOnly _returnvalue)
      (else
        (Input|SetInputModeUIOnly _returnvalue _maingui "DoNotLock")))))

(event Input|ActionEvents|InputActionDebug
  (params (Key :type Key%20Structure :default "None"))
  (:Pressed
    (Variables|Default|SetDebug (not (Variables|Default|GetDebug)))))

(event Input|AxisEvents|InputAxisMoveForward
  (params (AxisValue :type Float%20%28single-precision%29))
  (Pawn|Input|AddMovementInput (Math|Vector|GetForwardVector (Math|Rotator|MakeRotator 0.0 0.0 (.yaw (Pawn|GetControlRotation :!class /Script/Engine.Pawn)))) AxisValue false)
  (Variables|Default|SetMoveForward AxisValue))

(event Input|AxisEvents|InputAxisMoveRight
  (params (AxisValue :type Float%20%28single-precision%29))
  (Pawn|Input|AddMovementInput (Math|Vector|GetRightVector (Math|Rotator|MakeRotator 0.0 0.0 (.yaw (Pawn|GetControlRotation :!class /Script/Engine.Pawn)))) AxisValue false)
  (Variables|Default|SetMoveRight AxisValue))

(event Input|AxisEvents|InputAxisTurnRight
  (params (AxisValue :type Float%20%28single-precision%29))
  (Pawn|Input|AddControllerYawInput AxisValue))

(event Input|AxisEvents|InputAxisLookUp
  (params (AxisValue :type Float%20%28single-precision%29))
  (Pawn|Input|AddControllerPitchInput AxisValue))

(fn ConstructionScript)