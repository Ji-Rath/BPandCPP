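; Behavior Tree task that picks the next patrol destination along an NPC's assigned path spline.
; It increments the SplinePoint blackboard index, resetting to zero only when it exceeds the spline's point count.
; It writes that point's world X and Y to MoveLocation, keeping the NPC's current Z, then finishes successfully.
; A failed NPC cast stops execution without finishing the task.
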(event EventReceiveExecuteAI
  (params (OwnerController :type AI%20Controller%20Object%20Reference) (ControlledPawn :type Pawn%20Object%20Reference))
  (bind _splinepoint (Variables|Default|GetSplinePoint))
  (bind _returnvalue (Class|BTFunctionLibrary|GetBlackboardValueasInt _splinepoint))
  (bind _asnpc (Utilities|Casting|CastToNPC ControlledPawn))
  (bind _output_get (Variables|Default|SetPoint _returnvalue))
  (bind _result (Math|Integer|IncrementInt _output_get)
    (:%20%20
      (if (> _result (Spline|GetNumberOfSplinePoints (Variables|/Game/Blueprints/PathBP.PathBP_C|GetSpline (Variables|/Game/Blueprints/NPC.NPC_C|GetPath _asnpc))))
        (Variables|Default|SetPoint 0))
      (Class|BTFunctionLibrary|SetBlackboardValueasInt _splinepoint (Variables|Default|GetPoint))
      (AI|BehaviorTree|SetBlackboardValueasVector (Variables|Default|GetMoveLocation) (Math|Vector|MakeVector (.x (Spline|GetLocationatSplinePoint (Variables|/Game/Blueprints/PathBP.PathBP_C|GetSpline (Variables|/Game/Blueprints/NPC.NPC_C|GetPath _asnpc)) _returnvalue "World")) (.y (Spline|GetLocationatSplinePoint (Variables|/Game/Blueprints/PathBP.PathBP_C|GetSpline (Variables|/Game/Blueprints/NPC.NPC_C|GetPath _asnpc)) _returnvalue "World")) (.Z (Math|Vector|BreakVector (Transformation|GetActorLocation _asnpc)))))
      (AI|BehaviorTree|FinishExecute true))))